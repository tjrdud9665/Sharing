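; Tile generator Blueprint that builds a floor of randomly chosen static meshes in its construction script.
; GenerateTile adds spline points at fixed grid spacing, then adds a mesh component at each point using a random FloorType entry.
; The row index divides by NumOfTileX while the column wraps by NumOfTileY, so the grid layout assumes both counts are equal.
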(event EventBeginPlay)

(event Collision|EventActorBeginOverlap
  (params (OtherActor :type Actor%20Object%20Reference)))

(event EventTick
  (params (DeltaSeconds :type Float%20%28single-precision%29)))

(fn ConstructionScript
  (CallFunction|GenerateTile))

(fn GenerateTile
  (bind _floortype (Variables|Default|GetFloorType))
  (bind _numoftile_x (Variables|TileNum|GetNumOfTile_X))
  (bind _numoftile_y (Variables|TileNum|GetNumOfTile_Y))
  (bind _returnvalue (* _numoftile_y _numoftile_x))
  (for _index (range 0 _returnvalue)
    (Class|SplineComponent|AddPoint (Variables|Default|GetTileSpline) (Utilities|Struct|MakeSplinePoint (Math|Conversions|ToFloat(Integer) _index) (Math|Vector|MakeVector (Math|Conversions|ToFloat(Integer) (* (/ _index (Variables|TileNum|GetNumOfTile_X)) 2800)) (Math|Conversions|ToFloat(Integer) (* (Math|Integer|%(Integer) _index (Variables|TileNum|GetNumOfTile_Y)) 2800)) 0.0)) true))
  (for _index_2 (range 0 _returnvalue)
    (bind _returnvalue_2 (AddComponent|AddStaticMeshComponent false (Math|Transform|MakeTransform (Spline|GetLocationatSplinePoint (Variables|Default|GetTileSpline) _index_2 "Local") "0, 0, 0" "1,1,1")))
    (Components|StaticMesh|SetStaticMesh _returnvalue_2 (Utilities|Array|Get(acopy) _floortype (Math|Random|RandomInteger (Utilities|Array|Length _floortype))))))