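; Player controller Blueprint that creates the player's HUD frame and includes a hard-coded key for reducing health.
; On BeginPlay it creates a W_PlayerFrame widget, passes itself as TopDownController and adds it to the viewport.
; Pressing 1 subtracts a fixed amount of health through the character's UnitStatComponent, then pushes the current-to-max ratio straight into the health bar and prints it.
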(event EventBeginPlay
  (bind _returnvalue (UserInterface|CreateWidget "/Game/BluePrint/Widget/W_PlayerFrame.W_PlayerFrame_C" 0 self))
  (UserInterface|Viewport|AddtoViewport _returnvalue 0))

(event EventTick
  (params (DeltaSeconds :type Float%20%28single-precision%29)))

(event Input|KeyboardEvents|1
  (params (Key :type Key%20Structure))
  (bind _playercharacter (Variables|Default|GetPlayerCharacter))
  (bind _unitstatcomponent (Variables|/Script/First.BaseCharacter|GetUnitStatComponent _playercharacter))
  (bind _returnvalue (Default|GetStatInfo _unitstatcomponent "E_ST_HEALTH"))
  (bind (_maxvalue _currentvalue) (Utilities|Struct|BreakUnitStatInfo _returnvalue))
  (bind _returnvalue_2 (/ _currentvalue _maxvalue))
  (:Pressed
    (Default|SetUnitStat _unitstatcomponent "E_ST_HEALTH" (- _currentvalue 5e+01) _maxvalue)
    (Progress|SetPercent (Variables|/Script/First.PlayerFrame|GetHealthBar (stale EventBeginPlay _returnvalue)) _returnvalue_2)
    (Development|PrintString (Utilities|String|ToString(Float) _returnvalue_2))))

(fn ConstructionScript)